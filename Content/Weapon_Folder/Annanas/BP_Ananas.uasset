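; BP_Ananas is a pineapple-named proximity explosive that detonates when an enemy comes into range.
; An overlap on its box component reacts only to BP_CloseEnemie or BP_SpecialEnemie actors and prints a debug message.
; After a short delay, it plays an explosion sound, applies heavy radial damage around the box while ignoring the player character, then destroys itself.
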(event `self.Box_0.OnComponentBeginOverlap`
  (params (OverlappedComponent :type "PrimitiveComponent Object Reference") (OtherActor :type "Actor Object Reference") (OtherComp :type "PrimitiveComponent Object Reference") (OtherBodyIndex :type Integer) (bFromSweep :type Boolean) (SweepResult :type "HitResult Structure (by ref)"))
  (bind (_returnvalue_x _returnvalue_y _returnvalue_z) (`KismetMathLibrary.BreakVector` (`SceneComponent.K2_GetComponentLocation` (`self.Box_0`))))
  (cast `/Game/Enemie_Folder/Close_Enemie/BP_CloseEnemie` OtherActor
    (:`then`
      _)
    (:`CastFailed`
      (cast `/Game/Enemie_Folder/Spezial_Enemie/BP_SpecialEnemie` OtherActor)))
  (bind _output_get (set `self.Ignore` (`|MakeArray` (`self.PlayerChrater`) :!type "Actor Object Reference")))
  (`KismetSystemLibrary.PrintString` "Inside Area")
  (`KismetSystemLibrary.Delay` 0.5)
  (`GameplayStatics.PlaySound2D` "/Game/StarterContent/Audio/Explosion02.Explosion02" 1.0 1.0 0.0 null null)
  (`GameplayStatics.ApplyRadialDamage` 1000.0 (`KismetMathLibrary.MakeVector` _returnvalue_x _returnvalue_y _returnvalue_z) 200.0 null _output_get self null)
  (`self.K2_DestroyActor`))

(fn `UserConstructionScript`)