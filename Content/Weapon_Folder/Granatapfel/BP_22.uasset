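; BP_22 is an explosive actor in the Granatapfel weapon folder that detonates on impact.
; When its sphere component is hit, it plays an explosion sound and applies randomized radial damage around its static mesh, ignoring player 0.
; It then prints a debug message and destroys itself.
; Two duplicate, unconnected chains for direct damage to BP_CloseEnemie never run.
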(event `self.ReceiveBeginPlay`)

(event `self.Sphere_0.OnComponentHit`
  (params (HitComponent :type "PrimitiveComponent Object Reference") (OtherActor :type "Actor Object Reference") (OtherComp :type "PrimitiveComponent Object Reference") (NormalImpulse :type "Vector Structure") (Hit :type "HitResult Structure (by ref)"))
  (bind (_returnvalue_x _returnvalue_y _returnvalue_z) (`KismetMathLibrary.BreakVector` (`SceneComponent.K2_GetComponentLocation` (`self.StaticMesh`))))
  (`GameplayStatics.PlaySoundAtLocation` "/Game/StarterContent/Audio/Explosion01.Explosion01" (`SceneComponent.K2_GetComponentLocation` (`self.Sphere_0`)) (struct) 1.0 1.0 0.0 null null null null)
  (`GameplayStatics.ApplyRadialDamage` (`KismetMathLibrary.RandomFloatInRange` 110.0 120.0) (`KismetMathLibrary.MakeVector` _returnvalue_x _returnvalue_y _returnvalue_z) 900.0 null (`|MakeArray` (`self.Player_0`) :!type "Actor Object Reference") self null)
  (`KismetSystemLibrary.PrintString` "ImpactDamage")
  (`self.K2_DestroyActor`))

(fn `UserConstructionScript`)