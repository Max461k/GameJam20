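; BP_Shutgun is a short-lived actor that fires a shotgun blast of BP_ShootgunBullit projectiles from the player character.
; On BeginPlay it calls DestroyActor first, then runs the firing logic in the same event, so each instance is a single shot.
; A loop driven by ShotAmount spawns bullets at the player's ProjectileSpawn component, with SprayAngle spreading each direction around its forward vector using MaxAngle.
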(event `self.ReceiveBeginPlay`
  (`self.K2_DestroyActor`)
  (bind _asbp_player_charakter (cast `/Game/Player_Folder/Player_Input/PlayerBluePrint/BP_PlayerCharakter` (`GameplayStatics.GetPlayerCharacter` 0)))
  (for _ (range (+ (`self.ShotAmount`) 1))
    (bind (_returnvalue_location _returnvalue_rotation) (`KismetMathLibrary.BreakTransform` (`SceneComponent.K2_GetComponentToWorld` (`/Game/Player_Folder/Player_Input/PlayerBluePrint/BP_PlayerCharakter.ProjectileSpawn` _asbp_player_charakter))))
    (`|SpawnActorFromClass` "/Game/Weapon_Folder/shutgun/BP_ShootgunBullit.BP_ShootgunBullit_C" (`KismetMathLibrary.MakeTransform` _returnvalue_location (`/Game/Weapon_Folder/shutgun/BP_Bulitspray.SprayAngle` (`KismetMathLibrary.GetForwardVector` _returnvalue_rotation) (`self.MaxAngle`))) "AdjustIfPossibleButAlwaysSpawn" "MultiplyWithRoot" null null)))

(event `self.ReceiveTick`
  (params (DeltaSeconds :type "Float (single-precision)")))

(fn `UserConstructionScript`)