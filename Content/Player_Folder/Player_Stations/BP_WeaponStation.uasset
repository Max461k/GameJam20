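; BP_WeaponStation is a player station that grants a random special weapon when credit points meet the required amount.
; Box overlap toggles its prompt widget.
; Interacte draws from WeaponArray, sets the player's mesh via MeshMap, grants and removes that weapon, raises the requirement and boosts high score, without deducting credits here.
; FillArray appends the Original list to the pool, but nothing here calls it.
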(event `self.ReceiveBeginPlay`)

(event `self.Box.OnComponentBeginOverlap`
  (params (OverlappedComponent :type "PrimitiveComponent Object Reference") (OtherActor :type "Actor Object Reference") (OtherComp :type "PrimitiveComponent Object Reference") (OtherBodyIndex :type Integer) (bFromSweep :type Boolean) (SweepResult :type "HitResult Structure (by ref)"))
  (`SceneComponent.SetVisibility` (`self.Widget`) true false)
  (bind _asbp_player_charakter (cast `/Game/Player_Folder/Player_Input/PlayerBluePrint/BP_PlayerCharakter` OtherActor))
  (set `self.Player` _asbp_player_charakter))

(event `self.Box.OnComponentEndOverlap`
  (params (OverlappedComponent :type "PrimitiveComponent Object Reference") (OtherActor :type "Actor Object Reference") (OtherComp :type "PrimitiveComponent Object Reference") (OtherBodyIndex :type Integer))
  (`SceneComponent.SetVisibility` (`self.Widget`) false false))

(event `self.Interacte`
  (bind _asthis_game_mode (cast `/Game/Player_Folder/Player_Input/Gamemode/ThisGameMode` (`GameplayStatics.GetGameMode`)))
  (if (>= (`/Game/Player_Folder/Player_Input/Gamemode/ThisGameMode.CreditsPoints` _asthis_game_mode) (`self.RequiredWeaponPoints`))
    (`GameplayStatics.PlaySound2D` "/Engine/EditorSounds/GamePreview/EndPlayInEditor.EndPlayInEditor" 1.0 1.0 0.0 null null)
    (bind _asbp_player_charakter (cast `/Game/Player_Folder/Player_Input/PlayerBluePrint/BP_PlayerCharakter` (`GameplayStatics.GetPlayerCharacter` 0)))
    (bind _output_get (set `self.SelectedWeapon` (`KismetArrayLibrary.Array_Random` (`self.WeaponArray`))))
    (`StaticMeshComponent.SetStaticMesh` (`/Game/Player_Folder/Player_Input/PlayerBluePrint/BP_PlayerCharakter.SpecialWeaponMesh` _asbp_player_charakter) (`BlueprintMapLibrary.Map_Find` (`self.MeshMap`) _output_get))
    (`/Game/Player_Folder/Player_Input/PlayerBluePrint/BP_PlayerCharakter.Get SpecialWeapon` _asbp_player_charakter _output_get)
    (`KismetArrayLibrary.Array_RemoveItem` (`self.WeaponArray`) (`self.SelectedWeapon`))
    (set `/Game/Player_Folder/Player_Input/PlayerBluePrint/BP_PlayerCharakter.HasSpezialWeapon` true _asbp_player_charakter)
    (set `self.RequiredWeaponPoints` (+ (`self.RequiredWeaponPoints`) 50))
    (set `/Game/Player_Folder/Player_Input/Gamemode/ThisGameMode.HighScorePoints` (`KismetMathLibrary.Conv_Int64ToInt` (+ (`KismetMathLibrary.Round64` (* (`/Game/Player_Folder/Player_Input/Gamemode/ThisGameMode.HighScorePoints` _asthis_game_mode) 0.2)) (`/Game/Player_Folder/Player_Input/Gamemode/ThisGameMode.HighScorePoints` _asthis_game_mode))) _asthis_game_mode)))

(event `Fill Array`
  (for _array_element (`self.Original`)
    (`KismetArrayLibrary.Array_Add` (`self.WeaponArray`) _array_element)))

(event `self.ReceiveTick`
  (params (DeltaSeconds :type "Float (single-precision)")))

(fn `UserConstructionScript`)