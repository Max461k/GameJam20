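; BP_HealStation is a player station that sells a full heal for credits.
; A box overlap shows its widget and stores the player.
; Interacte plays a sound, then, if health is below 100 and the game mode has enough CreditsPoints, deducts the cost and restores health.
; Each purchase raises that station's next price and boosts HighScorePoints by a percentage of its current value.
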(event `self.ReceiveBeginPlay`
  (set `self.RequiredSkillPoints` 100))

(event `self.Box.OnComponentBeginOverlap`
  (params (OverlappedComponent :type "PrimitiveComponent Object Reference") (OtherActor :type "Actor Object Reference") (OtherComp :type "PrimitiveComponent Object Reference") (OtherBodyIndex :type Integer) (bFromSweep :type Boolean) (SweepResult :type "HitResult Structure (by ref)"))
  (`SceneComponent.SetVisibility` (`self.Widget`) true false)
  (bind _asbp_player_charakter (cast `/Game/Player_Folder/Player_Input/PlayerBluePrint/BP_PlayerCharakter` OtherActor))
  (set `self.Player` _asbp_player_charakter))

(event `self.Box.OnComponentEndOverlap`
  (params (OverlappedComponent :type "PrimitiveComponent Object Reference") (OtherActor :type "Actor Object Reference") (OtherComp :type "PrimitiveComponent Object Reference") (OtherBodyIndex :type Integer))
  (`SceneComponent.SetVisibility` (`self.Widget`) false false))

(event `/Game/Player_Folder/Player_Stations/InteracteInterface.Interacte`
  (`GameplayStatics.PlaySound2D` "/Game/Enemie_Folder/Sounds/heal_2.heal_2" 1.0 1.0 0.0 null null)
  (if (< (`/Game/Player_Folder/Player_Input/PlayerBluePrint/BP_PlayerCharakter.PlayerHealth` (`self.Player`)) 100.0)
    (bind _asthis_game_mode (cast `/Game/Player_Folder/Player_Input/Gamemode/ThisGameMode` (`GameplayStatics.GetGameMode`)))
    (if (>= (`/Game/Player_Folder/Player_Input/Gamemode/ThisGameMode.CreditsPoints` _asthis_game_mode) (`self.RequiredSkillPoints`))
      (set `/Game/Player_Folder/Player_Input/Gamemode/ThisGameMode.CreditsPoints` (- (`/Game/Player_Folder/Player_Input/Gamemode/ThisGameMode.CreditsPoints` _asthis_game_mode) (`self.RequiredSkillPoints`)) _asthis_game_mode)
      (set `/Game/Player_Folder/Player_Input/PlayerBluePrint/BP_PlayerCharakter.PlayerHealth` 100.0 (`self.Player`))
      (`KismetSystemLibrary.PrintString` "Wer das liest schuldet mir eine cola")
      (bind _output_get (set `self.RequiredSkillPoints` (+ (stale _output_get) 100)))
      (set `/Game/Player_Folder/Player_Input/Gamemode/ThisGameMode.HighScorePoints` (`KismetMathLibrary.Conv_Int64ToInt` (+ (`/Game/Player_Folder/Player_Input/Gamemode/ThisGameMode.HighScorePoints` _asthis_game_mode) (`KismetMathLibrary.Round64` (* (`/Game/Player_Folder/Player_Input/Gamemode/ThisGameMode.HighScorePoints` _asthis_game_mode) 0.2)))) _asthis_game_mode))
    (else
      (`KismetSystemLibrary.PrintString` "No need to heal"))))

(fn `UserConstructionScript`)