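; BP_EnemieSpawner spawns close-range enemies across the level's spawn points.
; On BeginPlay it registers itself with ThisGameMode as the EnemieSpawner reference.
; SpawnEnemies splits the requested count evenly over all BP_SpawnPoint actors, truncating each share, so any remainder is not spawned.
; Each BP_CloseEnemie spawns at its point's transform, adjusted for collision, is stored in EnemiesInLevel, and its array index is printed for debugging.
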(event `self.ReceiveBeginPlay`
  (bind _asthis_game_mode (cast `/Game/Player_Folder/Player_Input/Gamemode/ThisGameMode` (`GameplayStatics.GetGameMode`)))
  (set `/Game/Player_Folder/Player_Input/Gamemode/ThisGameMode.EnemieSpawner` self _asthis_game_mode))

(fn `Spawn Enemies`
  (params (count :type "Float (double-precision)"))
  (bind _outactors (`GameplayStatics.GetAllActorsOfClass` "/Game/Enemie_Folder/Close_Enemie/BP_SpawnPoint.BP_SpawnPoint_C"))
  (for _array_element _outactors
    (for _ (range 1 (+ (`KismetMathLibrary.FTrunc` (/ count (`KismetArrayLibrary.Array_Length` _outactors))) 1))
      (bind _returnvalue (`|SpawnActorFromClass` "/Game/Enemie_Folder/Close_Enemie/BP_CloseEnemie.BP_CloseEnemie_C" (`self.GetTransform` _array_element) "AdjustIfPossibleButAlwaysSpawn" "MultiplyWithRoot" null null))
      (bind _returnvalue_2 (`KismetArrayLibrary.Array_Add` (`self.EnemiesInLevel`) _returnvalue))
      (`KismetSystemLibrary.PrintString` (`KismetStringLibrary.Conv_IntToString` _returnvalue_2) true true (struct :`R` 1.0 :`G` 0.18486 :`A` 1.0)))))

(fn `UserConstructionScript`)