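; Special enemy for a round-based game that chases and melees the player, tracked in ThisGameMode's alive-enemy count.
; Each Tick reissues an AI move to the player; reaching them re-arms an attack flag, enabling delayed random damage with a round-scaled maximum.
; Incoming damage plays a hurt sound and lowers health until death.
; Death updates the game mode's counts, credits, high score and special-kill flag, checks kills, then destroys the actor.
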(event `self.ReceiveBeginPlay`
  (`|ExecutionSequence`
    (:`then_0`
      (bind _asthis_game_mode (cast `/Game/Player_Folder/Player_Input/Gamemode/ThisGameMode` (`GameplayStatics.GetGameMode`)))
      (`/Engine/EditorBlueprintResources/StandardMacros.IncrementInt` (`/Game/Player_Folder/Player_Input/Gamemode/ThisGameMode.AliveEnemies` _asthis_game_mode)))))

(event `self.ReceiveTick`
  (params (DeltaSeconds :type "Float (single-precision)"))
  (`self.FollowPlayer`))

(event `FollowPlayer`
  (`|AIMoveTo` self (`self.K2_GetActorLocation` (`GameplayStatics.GetPlayerCharacter` 0)) (`GameplayStatics.GetPlayerCharacter` 0) 80.0
    (:`then`
      (if (`self.CanAttack`)
        (set `self.CanAttack` false)
        (`KismetSystemLibrary.Delay` 0.3)
        (`KismetSystemLibrary.PrintText` "Attacking")
        (`GameplayStatics.ApplyDamage` (`GameplayStatics.GetPlayerCharacter` 0) (`KismetMathLibrary.RandomFloatInRange` 35.0 (+ (`/Game/Player_Folder/Player_Input/Gamemode/ThisGameMode.CurrentRound` (stale `self.ReceiveBeginPlay` _asthis_game_mode)) 45.0)) null self)
        (set `self.CanAttack` false)))
    (:`OnSuccess`
      (`KismetSystemLibrary.Delay` 0.2)
      (set `self.CanAttack` true))))

(event `self.ReceiveAnyDamage`
  (params (Damage :type "Float (single-precision)") (DamageType :type "DamageType Object Reference") (InstigatedBy :type "Controller Object Reference") (DamageCauser :type "Actor Object Reference"))
  (`GameplayStatics.PlaySound2D` "/Game/Sound_Folder/monster_hurt.monster_hurt" 1.0 1.0 0.0 null null)
  (set `self.EnemieHealth` (- (`self.EnemieHealth`) Damage))
  (if (<= (`self.EnemieHealth`) 0.0)
    (`self.OnEnemieDead`)
    (`GameplayStatics.PlaySound2D` "/Game/Sound_Folder/monsterdead.monsterdead" 1.0 1.0 0.0 null null)))

(event `OnEnemieDead`
  (bind _asthis_game_mode (cast `/Game/Player_Folder/Player_Input/Gamemode/ThisGameMode` (`GameplayStatics.GetGameMode`)))
  (`/Engine/EditorBlueprintResources/StandardMacros.DecrementInt` (`/Game/Player_Folder/Player_Input/Gamemode/ThisGameMode.AliveEnemies` _asthis_game_mode)
    (:`  `
      (bind _result (`/Engine/EditorBlueprintResources/StandardMacros.IncrementInt` (stale _output_get))
        (:`  `
          (bind _output_get (set `/Game/Player_Folder/Player_Input/Gamemode/ThisGameMode.EnemiesKilled` _result _asthis_game_mode))
          (set `/Game/Player_Folder/Player_Input/Gamemode/ThisGameMode.CreditsPoints` (+ 25 (`/Game/Player_Folder/Player_Input/Gamemode/ThisGameMode.CreditsPoints` _asthis_game_mode)) _asthis_game_mode)
          (set `/Game/Player_Folder/Player_Input/Gamemode/ThisGameMode.HighScorePoints` (+ (`/Game/Player_Folder/Player_Input/Gamemode/ThisGameMode.CreditsPoints` _asthis_game_mode) 10) _asthis_game_mode)
          (set `/Game/Player_Folder/Player_Input/Gamemode/ThisGameMode.IsSpezialEnemieKilled` true _asthis_game_mode)
          (`/Game/Player_Folder/Player_Input/Gamemode/ThisGameMode.Check_EnemiesKilled` _asthis_game_mode)
          (`self.K2_DestroyActor`))))))

(fn `UserConstructionScript`)